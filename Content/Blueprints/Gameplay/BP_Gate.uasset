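; BP_Gate is a gate actor that opens when its linked lever is activated.
; On BeginPlay it stores the gate model's closed position, computes an open position raised along Z, and binds OpenGate to the TargetLever's activation event.
; OpenGate prints a debug message and plays a timeline that lerps the model's relative location from closed to open, with no closing logic.
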(event Custom|OpenGate
  ;[0.15 0.15 0.15 0.5] Gate Opening Procedure (Clay)
  (Development|PrintString "Gate opens")
  (bind _alpha (Timeline|TL_RaiseGate Play) ; Add Effects and sounds off of the Finished Pin (Clay)
    (:Update
      (Transformation|SetRelativeLocation (Variables|Default|GetGateModel) (Math|Vector|Lerp(Vector) (Variables|Default|GetClosedGateLocation) (Variables|Default|GetOpenGateLocation) _alpha) false false))))

(event EventBeginPlay
  ;[0.15 0.15 0.15 0.5] Gate Location Setup and Dispatch Responder to the Set Lever (Clay)
  (bind _output_get (Variables|Default|SetClosedGateLocation (Variables|/Script/Engine.SceneComponent|GetRelativeLocation (Variables|Default|GetGateModel))))
  (Variables|Default|SetOpenGateLocation (+ _output_get "0.000000,0.000000,300.000000"))
  (EventDispatchers|BindEventtoOnLeverActivated (Variables|Default|GetTargetLever) (delegate Custom|OpenGate)))

(fn ConstructionScript)