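; BP_Panel_TEST is a work-in-progress interactable 3D gem panel that opens a gem-swapping UI.
; Interact creates WBP_GemSwap with the panel and the player's IdolRef as owners, then switches to UI-only input.
; UpdateGemSlot writes GemStorage, then spawns or destroys a BP_TriangleGem and reassigns TrianglePanelSlot.
; BeginPlay refreshes slot 0 from pre-assigned red or green gem instances, as only triangle gems are handled so far.
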(event Custom|UpdateGemSlot
  (params (slotIndex :type Integer) (newGemData :type S%20Gem%20Data%20Structure))
  (bind _gemstorage (Variables|Default|GetgemStorage))
  (bind _output (Utilities|Array|Get(acopy) _gemstorage slotIndex))
  (Utilities|Array|SetArrayElem _gemstorage slotIndex newGemData)
  ;[0.15 0.15 0.15 0.5] come back to this; spawning physical sprite actor on 3d panel
  (if (.IsValid (Utilities|Struct|BreakS_GemData _output))
    (bind _returnvalue (Game|SpawnActorfromClass "/Game/Blueprints/Gameplay/Gems/BP_TriangleGem.BP_TriangleGem_C" (Transformation|GetRelativeTransform (Variables|Default|GetTrianglePanelSlot self)) "Undefined" "MultiplyWithRoot" 0 _output 0))
    (bind _output_get (Variables|Default|SettriangleGem _returnvalue))
    (Variables|Default|SetTrianglePanelSlot (Variables|/Game/Blueprints/Gameplay/Gems/BP_TriangleGem.BP_TriangleGem_C|GetTriangleGemSprite _output_get))
    (else
      (Actor|DestroyActor (Variables|Default|GettriangleGem))
      (Variables|Default|SetTrianglePanelSlot 0))))

(event EventBeginPlay
  (for _array_element (Variables|Default|GetgemStorage) ; checks assigned gems at start and updates its gem storage info
    (if (and (.IsValid (Utilities|Struct|BreakS_GemData _array_element)) (Utilities|IsValid (.GemInstance (Utilities|Struct|BreakS_GemData _array_element))))
      (switch Utilities|FlowControl|Switch|SwitchonEColors (.Color (Utilities|Struct|BreakS_GemData _array_element)) ; just checking for triangle for now
        (:NewEnumerator0
          _)
        (:NewEnumerator1
          _))
      (bind _asbp_triangle_gem (Utilities|Casting|CastToBP_TriangleGem (.GemInstance (Utilities|Struct|BreakS_GemData _array_element))))
      (CallFunction|UpdateGemSlot 0 (Variables|/Game/Blueprints/Gameplay/Gems/BP_TriangleGem.BP_TriangleGem_C|GetgemData _asbp_triangle_gem)))))

(event EventInteract
  (params (Instigator :type Actor%20Object%20Reference))
  (bind _returnvalue (Game|GetPlayerController 0))
  (bind _asbp_first_person_character (Utilities|Casting|CastToBP_FirstPersonCharacter (Game|GetPlayerCharacter 0)))
  (Development|PrintString "panel felt you")
  (bind _returnvalue_2 (UserInterface|CreateWidget "/Game/Blueprints/UI/GemSwapping/WBP_GemSwap.WBP_GemSwap_C" _returnvalue self (Variables|/Game/Blueprints/Framework/BP_FirstPersonCharacter.BP_FirstPersonCharacter_C|GetidolRef _asbp_first_person_character)))
  (UserInterface|Viewport|AddtoViewport _returnvalue_2 0)
  (Input|SetInputModeUIOnly _returnvalue 0 "DoNotLock" false)
  (Variables|/Script/Engine.PlayerController|SetbShowMouseCursor _returnvalue true))

(fn ConstructionScript)