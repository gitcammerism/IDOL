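; Test trap actor that kills overlapping actors through their BP_Health component, filtered by the gems in its TrapPanel.
; On overlap, CanHitActor decides whether the actor is a valid target; an empty gem set hits anything.
; Only the triangle gem is evaluated, as a temporary measure: red targets BP_DemonAI and green targets BP_FirstPersonCharacter.
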(event Custom|CheckGemsPanel
  (params (targetActor :type Actor%20Object%20Reference))
  (bind _returnvalue (Actor|GetComponentbyClass targetActor "/Game/Blueprints/Gameplay/BP_Health.BP_Health_C"))
  (bind _output_get (Variables|Default|SettargetActor targetActor))
  (bind _canhit (CallFunction|CanHitActor _output_get))
  (if _canhit
    (Utilities|IsValid _returnvalue
      (:Is%20Valid
        (Default|Kill _returnvalue)))))

(event Collision|EventActorBeginOverlap
  (params (OtherActor :type Actor%20Object%20Reference))
  (CallFunction|CheckGemsPanel OtherActor))

(fn ConstructionScript)

(fn CanHitActor
  (params (targetActor :type Actor%20Object%20Reference))
  (bind _trappanel (Variables|Default|GettrapPanel))
  (bind _gemset (Variables|/Game/Developer/BP_Panel_TEST.BP_Panel_TEST_C|GetgemSet _trappanel))
  (bind (_triangle _circle _square) (Utilities|Struct|BreakS_GemSet _gemset))
  (bind _returnvalue (Utilities|IsValid _triangle))
  (LocalVariables|Settarget targetActor)
  (if (Math|Boolean|ORBoolean _returnvalue (Utilities|IsValid _circle) (Utilities|IsValid _square))
    (if _returnvalue ; temp; only checking for triangle for now
      (bind _asbp_triangle_gem (Utilities|Casting|CastToBP_TriangleGem _triangle))
      (switch Utilities|FlowControl|Switch|SwitchonETriangleColors (Variables|/Game/Blueprints/Gameplay/Gems/BP_TriangleGem.BP_TriangleGem_C|GettriangleColor _asbp_triangle_gem)
        (:NewEnumerator0
          (Utilities|Casting|CastToBP_DemonAI (LocalVariables|Gettarget)
            (:then
              _)
            (:CastFailed
              (return false))))
        (:NewEnumerator1
          (Utilities|Casting|CastToBP_FirstPersonCharacter (LocalVariables|Gettarget)
            (:then
              _)
            (:CastFailed
              (return false)))))
      (return true))
    (else
      (return true))))